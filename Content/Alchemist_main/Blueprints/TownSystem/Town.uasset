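; Town object for an alchemist game that simulates disease outbreaks in its population and pays the player gold for cures.
; Each simulated day, Tick applies deaths and spread, computes unrest, ages and prioritises each disease, then creates or updates priority-based reward Requests.
; Administer applies a Remedy's effects, shrinking, curing or adding infections by strength, paying out the request when a disease clears.
; SpawnDiseases seeds random outbreaks from the World's shuffled disease pool.
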(fn AddDisease
  (params (Disease :type Disease%20Object%20Reference) (Initial%20Infected :type Integer))
  (if (not (Utilities|Array|ContainsItem (Variables|Default|GetDiseases) Disease))
    (Utilities|Array|Add (Variables|Default|GetDiseases) Disease)
    (Utilities|Map|Add (Variables|Default|GetInfected) Disease Initial%20Infected)))

(fn Tick
  (LocalVariables|SetInitPop (Variables|Default|GetHealthyPopulation))
  ;[1 1 1] Kill some of the population based on the lethality of the disease
  (for _array_element (Variables|Default|GetDiseases)
    (if (.ReturnValue (Utilities|Map|Find (Variables|Default|GetInfected) _array_element))
      (Utilities|Map|Add (Variables|Default|GetInfected) _array_element (- (.Value (Utilities|Map|Find (Variables|Default|GetInfected) _array_element)) (Math|Float|Round (* (.Value (Utilities|Map|Find (Variables|Default|GetInfected) _array_element)) (Variables|/Game/Alchemist_main/Blueprints/TownSystem/Disease.Disease_C|GetLethality _array_element)))))
      (Variables|Default|SetDeadPopulation (+ (Math|Float|Round (* (.Value (Utilities|Map|Find (Variables|Default|GetInfected) _array_element)) (Variables|/Game/Alchemist_main/Blueprints/TownSystem/Disease.Disease_C|GetLethality _array_element))) (Variables|Default|GetDeadPopulation)))
      (else
        (Development|PrintString 0 "Error - Disease exists but is not in infected map"))))
  ;[1 1 1] Spread the Disease throughout the population (Maybe should do deaths first?)
  (for _array_element_2 (Variables|Default|GetDiseases)
    (Utilities|Map|Add (Variables|Default|GetInfected) _array_element_2 (Math|Float|Round (+ (* (Variables|Default|GetHealthyPopulation) (Variables|/Game/Alchemist_main/Blueprints/TownSystem/Disease.Disease_C|GetSpread _array_element_2)) (Math|Conversions|ToFloat(Integer) (.Value (Utilities|Map|Find (Variables|Default|GetInfected) _array_element_2))))))
    (Variables|Default|SetHealthyPopulation (- (Variables|Default|GetHealthyPopulation) (Math|Float|Round (* (Variables|Default|GetHealthyPopulation) (Variables|/Game/Alchemist_main/Blueprints/TownSystem/Disease.Disease_C|GetSpread _array_element_2))))))
  ;[1 1 1] Calculate the Towns Unrest for this day
  (for _array_element_3 (Variables|Default|GetDiseases)
    (bind _output_get (LocalVariables|SetTotalInfected (+ (LocalVariables|GetTotalInfected) (.Value (Utilities|Map|Find (Variables|Default|GetInfected) _array_element_3))))))
  (Variables|Default|SetUnrest (CallFunction|UnrestEquation _output_get))
  (LocalVariables|SetTotalInfected 0)
  ;[1 1 1] Set the priority of each disease, based on the equation
  (for _array_element_4 (Variables|Default|GetDiseases)
    (Math|Integer|IncrementInt (Variables|/Game/Alchemist_main/Blueprints/TownSystem/Disease.Disease_C|GetAge _array_element_4)
      (:%20%20
        (CallFunction|PriorityEquation _array_element_4 (/ (.Value (Utilities|Map|Find (Variables|Default|GetInfected) _array_element_4)) (Variables|Default|GetHealthyPopulation)))
        (CallFunction|GenerateRequest)))))

(fn Administer
  (params (Remedy :type Ingredients%20Base%20Object%20Reference))
  (bind _world (Variables|Default|GetWorld))
  (bind _infected (Variables|Default|GetInfected))
  (bind _infected_2 (Variables|Default|GetInfected))
  (bind _infected_3 (Variables|Default|GetInfected))
  (bind _infected_4 (Variables|Default|GetInfected))
  (bind _infected_5 (Variables|Default|GetInfected))
  (bind _requests (Variables|Default|GetRequests))
  (bind _requests_2 (Variables|Default|GetRequests))
  (bind _world_2 (Variables|Default|GetWorld))
  (bind _player_character (Variables|/Game/Alchemist_main/Blueprints/TownSystem/World.World_C|GetPlayer%20Character _world_2))
  (bind _player_character_2 (Variables|/Game/Alchemist_main/Blueprints/TownSystem/World.World_C|GetPlayer%20Character _world))
  (for _array_element (Variables|/Game/Alchemist_main/Blueprints/InteractableObjects/GrabbableObjects/Ingredients/IngredientsBase.IngredientsBase_C|GetEffects Remedy)
    (if (Variables|/Game/Alchemist_main/Blueprints/TownSystem/Effect.Effect_C|GetCures _array_element)
      (for _array_element_2 (Variables|Default|GetDiseases)
        (if (Utilities|Enum|Equal(Enum) (Variables|/Game/Alchemist_main/Blueprints/TownSystem/Disease.Disease_C|GetName _array_element_2) (Variables|/Game/Alchemist_main/Blueprints/TownSystem/Disease.Disease_C|GetName (Variables|/Game/Alchemist_main/Blueprints/TownSystem/Effect.Effect_C|GetDisease _array_element)))
          (LocalVariables|Setcontains true)))
      (if (== (Variables|/Game/Alchemist_main/Blueprints/TownSystem/Effect.Effect_C|GetStrength _array_element) 1)
        (if (LocalVariables|Getcontains)
          (if (<= (- (/ (.Value (Utilities|Map|Find _infected_4 (Variables|/Game/Alchemist_main/Blueprints/TownSystem/Effect.Effect_C|GetDisease _array_element))) 2) 10) 0)
            (Utilities|Array|RemoveItem (Variables|Default|GetDiseases) (Variables|/Game/Alchemist_main/Blueprints/TownSystem/Effect.Effect_C|GetDisease _array_element))
            (Variables|Default|SetHealthyPopulation (+ (Variables|Default|GetHealthyPopulation) (.Value (Utilities|Map|Find _infected_2 (Variables|/Game/Alchemist_main/Blueprints/TownSystem/Effect.Effect_C|GetDisease _array_element)))))
            (Utilities|Map|Remove _infected_2 (Variables|/Game/Alchemist_main/Blueprints/TownSystem/Effect.Effect_C|GetDisease _array_element))
            (Variables|/Game/Alchemist_main/Blueprints/MainCharacter.MainCharacter_C|SetGold _player_character (+ (Variables|/Game/Alchemist_main/Blueprints/MainCharacter.MainCharacter_C|GetGold _player_character) (Variables|/Game/Alchemist_main/Blueprints/TownSystem/Request.Request_C|GetReward (.Value (Utilities|Map|Find _requests_2 (Variables|/Game/Alchemist_main/Blueprints/TownSystem/Effect.Effect_C|GetDisease _array_element))))))
            (Utilities|Map|Remove _requests_2 (Variables|/Game/Alchemist_main/Blueprints/TownSystem/Effect.Effect_C|GetDisease _array_element))
            (LocalVariables|Setcontains false)
            (else
              (Utilities|Map|Add _infected_4 (Variables|/Game/Alchemist_main/Blueprints/TownSystem/Effect.Effect_C|GetDisease _array_element) (- (/ (.Value (Utilities|Map|Find _infected_4 (Variables|/Game/Alchemist_main/Blueprints/TownSystem/Effect.Effect_C|GetDisease _array_element))) 2) 10)))))
        (elif (LocalVariables|Getcontains)
          (Utilities|Array|RemoveItem (Variables|Default|GetDiseases) (Variables|/Game/Alchemist_main/Blueprints/TownSystem/Effect.Effect_C|GetDisease _array_element))
          (Variables|Default|SetHealthyPopulation (+ (Variables|Default|GetHealthyPopulation) (.Value (Utilities|Map|Find _infected_5 (Variables|/Game/Alchemist_main/Blueprints/TownSystem/Effect.Effect_C|GetDisease _array_element)))))
          (Utilities|Map|Remove _infected_5 (Variables|/Game/Alchemist_main/Blueprints/TownSystem/Effect.Effect_C|GetDisease _array_element))
          (Variables|/Game/Alchemist_main/Blueprints/MainCharacter.MainCharacter_C|SetGold _player_character_2 (+ (Variables|/Game/Alchemist_main/Blueprints/MainCharacter.MainCharacter_C|GetGold _player_character_2) (Variables|/Game/Alchemist_main/Blueprints/TownSystem/Request.Request_C|GetReward (.Value (Utilities|Map|Find _requests (Variables|/Game/Alchemist_main/Blueprints/TownSystem/Effect.Effect_C|GetDisease _array_element))))))
          (Utilities|Map|Remove _requests (Variables|/Game/Alchemist_main/Blueprints/TownSystem/Effect.Effect_C|GetDisease _array_element))
          (LocalVariables|Setcontains false)))
      (else
        (for _array_element_3 (Variables|Default|GetDiseases)
          (if (Utilities|Enum|Equal(Enum) (Variables|/Game/Alchemist_main/Blueprints/TownSystem/Disease.Disease_C|GetName _array_element_3) (Variables|/Game/Alchemist_main/Blueprints/TownSystem/Disease.Disease_C|GetName (Variables|/Game/Alchemist_main/Blueprints/TownSystem/Effect.Effect_C|GetDisease _array_element)))
            (LocalVariables|Setcontains true)))
        (if (== (Variables|/Game/Alchemist_main/Blueprints/TownSystem/Effect.Effect_C|GetStrength _array_element) 1)
          (if (LocalVariables|Getcontains)
            (Utilities|Map|Add _infected (Variables|/Game/Alchemist_main/Blueprints/TownSystem/Effect.Effect_C|GetDisease _array_element) (+ (.Value (Utilities|Map|Find _infected (Variables|/Game/Alchemist_main/Blueprints/TownSystem/Effect.Effect_C|GetDisease _array_element))) (Math|Float|Round (* (Variables|Default|GetHealthyPopulation) (Variables|Default|GetWeak%25)))))
            (Variables|Default|SetHealthyPopulation (- (Variables|Default|GetHealthyPopulation) (Math|Float|Round (* (Variables|Default|GetHealthyPopulation) (Variables|Default|GetWeak%25)))))
            (LocalVariables|Setcontains false)
            (else
              (Utilities|Map|Add (Variables|Default|GetInfected) (Variables|/Game/Alchemist_main/Blueprints/TownSystem/Effect.Effect_C|GetDisease _array_element) (Math|Float|Round (* (Variables|Default|GetHealthyPopulation) (Variables|Default|GetWeak%25))))
              (Variables|Default|SetHealthyPopulation (- (Variables|Default|GetHealthyPopulation) (Math|Float|Round (* (Variables|Default|GetHealthyPopulation) (Variables|Default|GetWeak%25)))))))
          (elif (LocalVariables|Getcontains)
            (Utilities|Map|Add _infected_3 (Variables|/Game/Alchemist_main/Blueprints/TownSystem/Effect.Effect_C|GetDisease _array_element) (+ (.Value (Utilities|Map|Find _infected_3 (Variables|/Game/Alchemist_main/Blueprints/TownSystem/Effect.Effect_C|GetDisease _array_element))) (Math|Float|Round (* (Variables|Default|GetHealthyPopulation) (Variables|Default|GetStrong%25)))))
            (Variables|Default|SetHealthyPopulation (- (Variables|Default|GetHealthyPopulation) (Math|Float|Round (* (Variables|Default|GetHealthyPopulation) (Variables|Default|GetStrong%25)))))
            (LocalVariables|Setcontains false)
            (else
              (Utilities|Map|Add (Variables|Default|GetInfected) (Variables|/Game/Alchemist_main/Blueprints/TownSystem/Effect.Effect_C|GetDisease _array_element) (Math|Float|Round (* (Variables|Default|GetHealthyPopulation) (Variables|Default|GetStrong%25))))
              (Variables|Default|SetHealthyPopulation (- (Variables|Default|GetHealthyPopulation) (Math|Float|Round (* (Variables|Default|GetHealthyPopulation) (Variables|Default|GetStrong%25))))))))))))

(fn GenerateRequest
  (Development|PrintString 0 "Generated Reqs")
  (for _array_element (Variables|Default|GetDiseases)
    (if (.ReturnValue (Utilities|Map|Find (Variables|Default|GetRequests) _array_element))
      (if (!= (Variables|/Game/Alchemist_main/Blueprints/TownSystem/Disease.Disease_C|GetPriority _array_element) (Variables|/Game/Alchemist_main/Blueprints/TownSystem/Request.Request_C|GetPriority (.Value (Utilities|Map|Find (Variables|Default|GetRequests) _array_element))))
        (Variables|/Game/Alchemist_main/Blueprints/TownSystem/Request.Request_C|SetPriority (.Value (Utilities|Map|Find (Variables|Default|GetRequests) _array_element)) (Variables|/Game/Alchemist_main/Blueprints/TownSystem/Disease.Disease_C|GetPriority _array_element))
        (Variables|/Game/Alchemist_main/Blueprints/TownSystem/Request.Request_C|SetReward (.Value (Utilities|Map|Find (Variables|Default|GetRequests) _array_element)) (Math|Float|Round (CallFunction|RewardEquation _array_element)))
        (Variables|/Game/Alchemist_main/Blueprints/TownSystem/Request.Request_C|SetInfected (.Value (Utilities|Map|Find (Variables|Default|GetRequests) _array_element)) (.Value (Utilities|Map|Find (Variables|Default|GetInfected) _array_element))))
      (else
        (bind _returnvalue (Game|ConstructObjectfromClass "/Game/Alchemist_main/Blueprints/TownSystem/Request.Request_C" "/Game/Alchemist_main/Blueprints/TownSystem/World.World" self _array_element (Math|Float|Round (CallFunction|RewardEquation _array_element)) (Variables|/Game/Alchemist_main/Blueprints/TownSystem/Disease.Disease_C|GetPriority _array_element) (.Value (Utilities|Map|Find (Variables|Default|GetInfected) _array_element))))
        (Utilities|Map|Add (Variables|Default|GetRequests) _array_element _returnvalue)))))

(fn RewardEquation
  (params (Disease :type Disease%20Object%20Reference))
  (return (* (Variables|/Game/Alchemist_main/Blueprints/TownSystem/Disease.Disease_C|GetPriority Disease) 0.75)))

(fn UnrestEquation
  (params (TotalInfected :type Integer))
  (return (Math|Conversions|ToFloat(Integer) (* (/ TotalInfected (Variables|Default|GetHealthyPopulation)) (Variables|Default|GetDeadPopulation)))))

(fn PriorityEquation
  (params (Disease :type Disease%20Object%20Reference) (Infected/Healthy :type Integer))
  (Variables|/Game/Alchemist_main/Blueprints/TownSystem/Disease.Disease_C|SetPriority Disease (Math|Float|Round (* (+ (Variables|/Game/Alchemist_main/Blueprints/TownSystem/Disease.Disease_C|GetAge Disease) 1) (* (+ Infected/Healthy 1) (+ (* 100 (Variables|/Game/Alchemist_main/Blueprints/TownSystem/Disease.Disease_C|GetLethality Disease)) (* 100 (Variables|/Game/Alchemist_main/Blueprints/TownSystem/Disease.Disease_C|GetSpread Disease)))))))
  (Development|PrintString 0 "priority set"))

(fn SpawnDiseases
  (params (MaxNewDiseases :type Integer))
  (bind _returnvalue (Math|Random|RandomIntegerinRange 1 15))
  (bind _world (Variables|Default|GetWorld))
  (bind _diseases (Variables|/Game/Alchemist_main/Blueprints/TownSystem/World.World_C|GetDiseases _world))
  (Utilities|Array|Shuffle _diseases)
  (for _array_element _diseases
    (if (< (LocalVariables|GetCurDiseasesAdded) MaxNewDiseases)
      (if (< (Math|Random|RandomIntegerinRange 0 100) (Math|Float|Truncate (* 100 (Variables|/Game/Alchemist_main/Blueprints/TownSystem/Disease.Disease_C|GetProbability _array_element))))
        (Math|Integer|IncrementInt (LocalVariables|GetCurDiseasesAdded)
          (:%20%20
            (if (> _returnvalue (Variables|Default|GetHealthyPopulation))
              (CallFunction|AddDisease _array_element (Variables|Default|GetHealthyPopulation))
              (else
                (CallFunction|AddDisease _array_element _returnvalue)))))))))