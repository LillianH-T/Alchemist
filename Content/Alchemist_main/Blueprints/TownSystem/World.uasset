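; World actor for the alchemist game's town system that owns the towns and diseases and serves as the interaction point for the town screen.
; On BeginPlay it constructs three Town objects with condition artwork, builds a catalogue of Disease objects, seeds starting infections and caches the player character.
; Interact opens the Town_UI widget with cursor and UI-only input.
; A helper derives a maximum disease value that grows with the day count.
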(event EventBeginPlay
  (CallFunction|MakeTowns)
  (CallFunction|MakeDiseases)
  (bind _asmain_character (Utilities|Casting|CastToMainCharacter (Game|GetPlayerCharacter 0)))
  (Variables|Default|SetPlayer%20Character _asmain_character))

(event Collision|EventActorBeginOverlap
  (params (OtherActor :type Actor%20Object%20Reference))
  (|CallParentFunction OtherActor) ; This node is disabled and will not be called.\nDrag off pins to build functionality.
)

(event EventTick
  (params (DeltaSeconds :type Float%20%28single-precision%29))
  (|CallParentFunction DeltaSeconds) ; This node is disabled and will not be called.\nDrag off pins to build functionality.
)

(fn ConstructionScript
  (|CallParentFunction))

(fn MakeTowns
  (bind _self self)
  (bind _self_2 self)
  (bind _self_3 self)
  (bind _returnvalue (Game|ConstructObjectfromClass "/Game/Alchemist_main/Blueprints/TownSystem/Town.Town_C" _self_2 _self_2 5000 "Sandland" (Class|WidgetBlueprintLibrary|MakeBrushfromTexture "/Game/Geometry/Town_maps/sandland/sandFull.sandFull") (Class|WidgetBlueprintLibrary|MakeBrushfromTexture "/Game/Geometry/Town_maps/sandland/sandMid.sandMid") (Class|WidgetBlueprintLibrary|MakeBrushfromTexture "/Game/Geometry/Town_maps/sandland/sandDest.sandDest")))
  (Utilities|Array|Add (Variables|Default|GetTowns) _returnvalue)
  (bind _returnvalue_2 (Game|ConstructObjectfromClass "/Game/Alchemist_main/Blueprints/TownSystem/Town.Town_C" _self_3 _self_3 500 "Iceland" (Class|WidgetBlueprintLibrary|MakeBrushfromTexture "/Game/Geometry/Town_maps/frostland/iceFull.iceFull") (Class|WidgetBlueprintLibrary|MakeBrushfromTexture "/Game/Geometry/Town_maps/frostland/iceMid.iceMid") (Class|WidgetBlueprintLibrary|MakeBrushfromTexture "/Game/Geometry/Town_maps/frostland/iceDest.iceDest")))
  (Utilities|Array|Add (Variables|Default|GetTowns) _returnvalue_2)
  (bind _returnvalue_3 (Game|ConstructObjectfromClass "/Game/Alchemist_main/Blueprints/TownSystem/Town.Town_C" _self _self 2000 "Treeland" (Class|WidgetBlueprintLibrary|MakeBrushfromTexture "/Game/Geometry/Town_maps/treeland/treeFull.treeFull") (Class|WidgetBlueprintLibrary|MakeBrushfromTexture "/Game/Geometry/Town_maps/treeland/treeMid.treeMid") (Class|WidgetBlueprintLibrary|MakeBrushfromTexture "/Game/Geometry/Town_maps/treeland/treeDest.treeDest")))
  (Utilities|Array|Add (Variables|Default|GetTowns) _returnvalue_3))

(fn MakeDiseases
  (bind _diseases (Variables|Default|GetDiseases))
  (bind _towns (Variables|Default|GetTowns))
  (bind _output (Utilities|Array|Get(acopy) _towns 1))
  (CallFunction|CreateDisease "Vomiting" 0.2 0.1 0.0)
  (CallFunction|CreateDisease "Itching" 0.1 0.1 0.0)
  (CallFunction|CreateDisease "Rash" 0.2 0.0 0.0)
  (CallFunction|CreateDisease "Aching" 0.05 0.0 0.0)
  (CallFunction|CreateDisease "Nausea" 0.1 0.0 0.0)
  (CallFunction|CreateDisease "Stoneskin" 0.1 0.15 0.1)
  (CallFunction|CreateDisease "Flametongue" 0.3 0.15 0.0)
  (CallFunction|CreateDisease "Swift Flu" 0.4 0.2 0.0)
  (CallFunction|CreateDisease "Vorgar's Mark" 0.1 0.05 0.2)
  (CallFunction|CreateDisease "Titan's Wrath" 0.3 0.01 0.4)
  (CallFunction|CreateDisease "Crawling Death" 0.1 0.02 0.5)
  (CallFunction|CreateDisease "Burning Plague" 0.55 0.01 0.3)
  ;[1 1 1] Initialise the towns with some diseases
  (Default|AddDisease (Utilities|Array|Get(acopy) _towns) (Utilities|Array|Get(acopy) _diseases) 3)
  (Default|AddDisease _output (Utilities|Array|Get(acopy) _diseases 1) 6)
  (Default|AddDisease _output (Utilities|Array|Get(acopy) _diseases 2) 9)
  (Default|AddDisease (Utilities|Array|Get(acopy) _towns 2) (Utilities|Array|Get(acopy) _diseases 3) 12))

(fn Interact
  (params (PlayerCharacter :type Main%20Character%20Object%20Reference) (InteractLocation :type Vector :default "0, 0, 0"))
  (bind _returnvalue (Game|GetPlayerController 0))
  ;[1 1 1] makes the shop widget
  (bind _returnvalue_2 (UserInterface|CreateWidget "/Game/Alchemist_main/Blueprints/TownSystem/Town_UI/town_UI.town_UI_C" 0 self))
  (UserInterface|Viewport|AddtoViewport _returnvalue_2 0)
  ;[1 1 1] Displays the mouse cursor and sets input to UI only
  (Input|SetInputModeUIOnly _returnvalue _returnvalue_2 "DoNotLock")
  (Variables|/Script/Engine.PlayerController|SetbShowMouseCursor _returnvalue true))

(fn MaxDiseaseEquation
  (return (+ (/ (Variables|Default|GetDay) 2) 1)))

(fn CreateDisease
  (params (Name :type String) (Spreadability :type Float%20%28single-precision%29) (Probability :type Float%20%28single-precision%29) (Lethality :type Float%20%28single-precision%29))
  (bind _returnvalue (Game|ConstructObjectfromClass "/Game/Alchemist_main/Blueprints/TownSystem/Disease.Disease_C" self Name Spreadability Probability Lethality))
  (Utilities|Array|Add (Variables|Default|GetDiseases) _returnvalue))