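; PackageBox is a delivery box that sends the ingredients placed inside it to a town when the day ends.
; On BeginPlay it binds to the Bed's EndDay dispatcher.
; When that fires, it gathers IngredientsBase actors overlapping its Box component, administers each to the World actor's town at TownIndex, then destroys them.
; The test event, CallGet and their debug wiring are unused leftovers.
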(event Custom|test)

(event Custom|End%20Day_Event_0
  (CallFunction|GetObjects)
  (CallFunction|AdministerContents)
  (CallFunction|EmptyBox))

(event EventBeginPlay
  (bind _returnvalue (Actor|GetActorOfClass "/Game/Alchemist_main/Blueprints/InteractableObjects/Bed.Bed_C"))
  (EventDispatchers|AssignEndDay _returnvalue (delegate Custom|End%20Day_Event_0)))

(fn ConstructionScript)

(fn GetObjects
  (bind _box (Variables|Default|GetBox))
  (bind _returnarray (Variables|Default|GetReturnArray))
  (Utilities|Array|Clear (Variables|Default|GetReturnArray))
  (bind _outactors (Collision|ComponentOverlapActors _box (Transformation|GetWorldTransform _box) (Utilities|Array|MakeArray "ObjectTypeQuery2" "ObjectTypeQuery1" "ObjectTypeQuery3" "ObjectTypeQuery4") "/Game/Alchemist_main/Blueprints/InteractableObjects/GrabbableObjects/Ingredients/IngredientsBase.IngredientsBase_C"))
  (for _array_element _outactors
    (bind _asingredients_base (Utilities|Casting|CastToIngredientsBase _array_element))
    (Utilities|Array|Add _returnarray _asingredients_base))
  (return _returnarray))

(fn CallGet
  ;[1 1 1] Test function
  (bind _allobjects (CallFunction|GetObjects))
  (Development|PrintString (Utilities|String|ToString(Integer) (Utilities|Array|Length _allobjects)))
  (Development|PrintString "Hello"))

(fn EmptyBox
  (bind _returnarray (Variables|Default|GetReturnArray))
  (for _array_element _returnarray
    (Actor|DestroyActor _array_element))
  (Utilities|Array|Clear _returnarray))

(fn AdministerContents
  (bind _returnvalue (Actor|GetActorOfClass "/Game/Alchemist_main/Blueprints/TownSystem/World.World_C"))
  (for _array_element (Variables|Default|GetReturnArray)
    (Default|Administer (Utilities|Array|Get(acopy) (Variables|/Game/Alchemist_main/Blueprints/TownSystem/World.World_C|GetTowns _returnvalue) (Variables|Default|GetTownIndex)) _array_element)))