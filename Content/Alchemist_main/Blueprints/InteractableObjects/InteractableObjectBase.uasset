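; InteractableObjectBase is a base Blueprint for objects the player can look at and interact with.
; LookAt toggles an outline by setting custom depth rendering and a stencil value on every primitive component, clearing both when the object leaves view.
; Interact takes the player character and a location but is empty here, as are Tick and the construction script.
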(event EventBeginPlay)

(event Collision|EventActorBeginOverlap
  (params (OtherActor :type Actor%20Object%20Reference)))

(event EventTick
  (params (DeltaSeconds :type Float%20%28single-precision%29)))

(fn ConstructionScript)

(fn Interact
  (params (PlayerCharacter :type Main%20Character%20Object%20Reference) (InteractLocation :type Vector)))

(fn Lookat
  (params (InView :type Boolean))
  (if InView
    ;[1 1 1] Enable outline
    (for _array_element (Actor|GetComponentsByClass "/Script/Engine.PrimitiveComponent")
      (bind _asprimitive_component (Utilities|Casting|CastToPrimitiveComponent _array_element))
      (Rendering|SetRenderCustomDepth _asprimitive_component true)
      (Rendering|SetCustomDepthStencilValue _asprimitive_component 2))
    (else
      ;[1 1 1] Enable outline
      (for _array_element_2 (Actor|GetComponentsByClass "/Script/Engine.PrimitiveComponent")
        (bind _asprimitive_component_2 (Utilities|Casting|CastToPrimitiveComponent _array_element_2))
        (Rendering|SetRenderCustomDepth _asprimitive_component_2 false)
        (Rendering|SetCustomDepthStencilValue _asprimitive_component_2 0)))))

(fn Tick)