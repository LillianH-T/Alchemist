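; Interactable ingredient book actor that opens the player's paged ingredient book UI.
; Its Interact function creates a Paged_ingredient_book widget, adds it to the viewport, then switches the first player controller to UI-only input focused on that widget and shows the mouse cursor.
; Each interaction creates a fresh widget, and the event graph holds only disabled default events.
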(event EventBeginPlay
  (|CallParentFunction) ; This node is disabled and will not be called.\nDrag off pins to build functionality.
)

(event Collision|EventActorBeginOverlap
  (params (OtherActor :type Actor%20Object%20Reference))
  (|CallParentFunction OtherActor) ; This node is disabled and will not be called.\nDrag off pins to build functionality.
)

(event EventTick
  (params (DeltaSeconds :type Float%20%28single-precision%29))
  (|CallParentFunction DeltaSeconds) ; This node is disabled and will not be called.\nDrag off pins to build functionality.
)

(fn ConstructionScript
  (|CallParentFunction))

(fn Interact
  (params (PlayerCharacter :type Main%20Character%20Object%20Reference) (InteractLocation :type Vector :default "0, 0, 0"))
  (bind _returnvalue (Game|GetPlayerController 0))
  ;[1 1 1] makes the ingredient book widget
  (bind _returnvalue_2 (UserInterface|CreateWidget "/Game/Alchemist_main/Blueprints/UISystem/Ingredient_book_ui/Paged_ingredient_book.Paged_ingredient_book_C"))
  (UserInterface|Viewport|AddtoViewport _returnvalue_2 0)
  ;[1 1 1] Displays the mouse cursor and sets input to UI only
  (Input|SetInputModeUIOnly _returnvalue _returnvalue_2 "DoNotLock")
  (Variables|/Script/Engine.PlayerController|SetbShowMouseCursor _returnvalue true))