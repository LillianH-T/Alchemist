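; Interactable cauldron where the player mixes held ingredients into a coloured liquid and transfers it to and from a Flask.
; Interact fills an empty flask with the mixed colour and accumulated effects, then resets the cauldron.
; Full flasks pour in and other ingredients are destroyed, both appending their effects.
; A dynamic material shows the colour, lerped by ingredient count so newer additions weigh increasingly heavily, despite the intended equal weighting.
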(event EventBeginPlay
  (|CallParentFunction)
  ;[1 1 1] Sets up dynamic liquid colouring so that the liquid can change when each ingredient is added
  (bind _returnvalue (Rendering|Material|CreateDynamicMaterialInstance (Variables|Default|GetLiquid) 0 "/Game/StarterContent/Materials/M_Water_Lake.M_Water_Lake" "None" :!class /Script/Engine.PrimitiveComponent))
  (Variables|Default|SetLiquidMat _returnvalue)
  (bind _output_get (Variables|Default|SetClearLiquidColor "(R=0.585538,G=0.783837,B=1.000000,A=0.777000)"))
  (bind _output_get_2 (Variables|Default|SetMixedLiquidColor _output_get))
  (Rendering|Material|SetVectorParameterValue (Variables|Default|GetLiquidMat) "Color" _output_get_2 :!class /Script/Engine.MaterialInstanceDynamic)
  (Audio|PlaySoundatLocation "/Game/Alchemist_main/Sound/SFX/bubbling.bubbling" (Transformation|GetActorLocation) "0, 0, 0" 1.0 1.0 0.0 0 0 0))

(event Collision|EventActorBeginOverlap
  (params (OtherActor :type Actor%20Object%20Reference))
  (|CallParentFunction OtherActor) ; This node is disabled and will not be called.\nDrag off pins to build functionality.
)

(event EventTick
  (params (DeltaSeconds :type Float%20%28single-precision%29))
  (|CallParentFunction DeltaSeconds) ; This node is disabled and will not be called.\nDrag off pins to build functionality.
)

(fn ConstructionScript
  (|CallParentFunction))

(fn UpdateLiquidColor
  (params (Color :type Linear%20Color%20Structure))
  (bind _numingredients (Variables|Default|GetNumIngredients))
  (bind _returnvalue (Math|Conversions|ToFloat(Integer) _numingredients))
  (bind _output_get (Variables|Default|SetMixedLiquidColor (Math|Color|Lerp(LinearColor) (Variables|Default|GetMixedLiquidColor) Color (/ _returnvalue (+ _returnvalue 1.0)))))
  (Rendering|Material|SetVectorParameterValue (Variables|Default|GetLiquidMat) "Color" _output_get :!class /Script/Engine.MaterialInstanceDynamic))

(fn Interact
  (params (PlayerCharacter :type Main%20Character%20Object%20Reference) (InteractLocation :type Vector :default "0, 0, 0"))
  (bind _heldobject (Variables|/Game/Alchemist_main/Blueprints/MainCharacter.MainCharacter_C|GetHeldObject PlayerCharacter))
  (|CallParentFunction PlayerCharacter InteractLocation)
  (if (Utilities|IsValid _heldobject)
    (bind _asflask (Utilities|Casting|CastToFlask _heldobject)
      (:then
        ;[1 1 1] If interacted with the flask, check if its full, if it is, empty the contents into the cauldron, otherwise empty the caudron into the flask
        (if (Variables|/Game/Alchemist_main/Blueprints/InteractableObjects/GrabbableObjects/Ingredients/Flask.Flask_C|GetIsEmpty _asflask)
          (Default|FillFlask _asflask (Variables|Default|GetMixedLiquidColor) (Variables|Default|GetEffects))
          (CallFunction|EmptyCauldron)
          (else
            (CallFunction|AddIngredient _asflask)))
        (Audio|PlaySoundatLocation "/Game/Alchemist_main/Sound/SFX/pour.pour" (Transformation|GetActorLocation) "0, 0, 0" 2.0 1.0 0.0 "/Game/Alchemist_main/Blueprints/InteractableObjects/CauldronAttenuation.CauldronAttenuation" 0 0))
      (:CastFailed
        ;[1 1 1] For ingredients that aren't the flask, just add the ingredient to the cauldron
        (bind _asingredients_base (Utilities|Casting|CastToIngredientsBase _heldobject))
        (CallFunction|AddIngredient _asingredients_base)))))

(fn AddIngredient
  (params (Ingredient :type Ingredients%20Base%20Object%20Reference))
  (Rendering|SetVisibility (Variables|Default|GetLiquid) true false)
  (Variables|Default|SetNumIngredients (+ (Variables|Default|GetNumIngredients) 1))
  (CallFunction|UpdateLiquidColor (Variables|/Game/Alchemist_main/Blueprints/InteractableObjects/GrabbableObjects/Ingredients/IngredientsBase.IngredientsBase_C|GetLiquidColor Ingredient))
  (Utilities|Array|AppendArray (Variables|Default|GetEffects) (Variables|/Game/Alchemist_main/Blueprints/InteractableObjects/GrabbableObjects/Ingredients/IngredientsBase.IngredientsBase_C|GetEffects Ingredient))
  (bind _asflask (Utilities|Casting|CastToFlask Ingredient)
    (:then
      (Default|EmptyFlask _asflask))
    (:CastFailed
      (Actor|DestroyActor Ingredient))))

(fn EmptyCauldron
  (Rendering|SetVisibility (Variables|Default|GetLiquid) false false)
  (Utilities|Array|Clear (Variables|Default|GetEffects))
  (Variables|Default|SetNumIngredients 0)
  (Variables|Default|SetMixedLiquidColor (Variables|Default|GetClearLiquidColor)))