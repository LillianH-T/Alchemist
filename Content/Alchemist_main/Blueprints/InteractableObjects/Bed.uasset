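; Interactable bed that ends the day and serves as the game's day-advance and game-over check.
; Interact cycles the music, calls EndDay, increments the World actor's day, ticks towns and spawns diseases, then compares summed unrest to the limit.
; Exceeding it shows the final screen; otherwise interactable objects tick and a timed camera fade leads to town and shop widgets.
; ExitBed fades back in with birdsong before returning the view to the player.
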(event EventBeginPlay
  (|CallParentFunction) ; This node is disabled and will not be called.\nDrag off pins to build functionality.
)

(event Collision|EventActorBeginOverlap
  (params (OtherActor :type Actor%20Object%20Reference))
  (|CallParentFunction OtherActor) ; This node is disabled and will not be called.\nDrag off pins to build functionality.
)

(event EventTick
  (params (DeltaSeconds :type Float%20%28single-precision%29))
  (|CallParentFunction DeltaSeconds) ; This node is disabled and will not be called.\nDrag off pins to build functionality.
)

(fn ConstructionScript
  (|CallParentFunction))

(fn Interact
  (params (PlayerCharacter :type Main%20Character%20Object%20Reference) (InteractLocation :type Vector :default "0, 0, 0"))
  ;[1 1 1] Queue next background music song in teh playlist
  (bind _output_get (Variables|/Game/Alchemist_main/Blueprints/MainCharacter.MainCharacter_C|SetsongNum PlayerCharacter (Math|Integer|%(Integer) (+ (Variables|/Game/Alchemist_main/Blueprints/MainCharacter.MainCharacter_C|GetsongNum PlayerCharacter) 1) 5)))
  (Effects|Components|ParticleSystem|SetIntParameter (Variables|/Game/Alchemist_main/Blueprints/MainCharacter.MainCharacter_C|GetMusic PlayerCharacter) "songNum" _output_get)
  (Default|CallEndDay)
  (bind _returnvalue (Actor|GetActorOfClass "/Game/Alchemist_main/Blueprints/TownSystem/World.World_C"))
  (Math|Integer|IncrementInt (Variables|/Game/Alchemist_main/Blueprints/TownSystem/World.World_C|GetDay _returnvalue)
    (:%20%20
      (bind _returnvalue_2 (Actor|GetActorOfClass "/Game/Alchemist_main/Blueprints/TownSystem/World.World_C"))
      (LocalVariables|Settotal%20unrest 0)
      (for _array_element (Variables|/Game/Alchemist_main/Blueprints/TownSystem/World.World_C|GetTowns _returnvalue_2)
        ;[1 1 1] Rolls for new diseases - the amount of max diseases
        (Default|Tick _array_element)
        (Default|SpawnDiseases _array_element (Default|MaxDiseaseEquation _returnvalue_2))
        ;[1 1 1] update total unrest
        (LocalVariables|Settotal%20unrest (+ (LocalVariables|Gettotal%20unrest) (Math|Float|Truncate (Variables|/Game/Alchemist_main/Blueprints/TownSystem/Town.Town_C|GetUnrest _array_element)))))
      ;[1 1 1] Checks game over
      (bind _game_over (CallFunction|CheckGameOver (LocalVariables|Gettotal%20unrest)))
      (if (not _game_over)
        ;[1 1 1] Call tick function on each interactable object
        (bind _outactors (Actor|GetAllActorsOfClass "/Game/Alchemist_main/Blueprints/InteractableObjects/InteractableObjectBase.InteractableObjectBase_C"))
        (for _array_element_2 _outactors
          ;;[1 1 1] This is needed incase the object is "pending kill"
          (if (Utilities|IsValid _array_element_2)
            (Default|Tick _array_element_2)))
        (CallFunction|CreateSleepMenus)))))

(fn DisplayTown
  (bind _returnvalue (Game|GetPlayerController 0))
  ;[1 1 1] Sets the sleep widgets
  ;;[1 1 1] sets up town ui
  (bind _returnvalue_2 (Actor|GetActorOfClass "/Game/Alchemist_main/Blueprints/TownSystem/World.World_C"))
  (bind _returnvalue_3 (UserInterface|CreateWidget "/Game/Alchemist_main/Blueprints/TownSystem/Town_UI/town_UI.town_UI_C" 0 _returnvalue_2))
  (UserInterface|Viewport|AddtoViewport _returnvalue_3 0)
  (Input|SetInputModeUIOnly _returnvalue _returnvalue_3 "DoNotLock")
  (EventDispatchers|BindEventtoExitClicked (Variables|/Game/Alchemist_main/Blueprints/TownSystem/Town_UI/town_UI.town_UI_C|GetExitButton_516 _returnvalue_3) (EventDispatchers|CreateEvent :!event ExitBed))
  (Variables|/Script/Engine.PlayerController|SetbShowMouseCursor _returnvalue true)
  ;;[1 1 1] sets up shop access from sleep menu
  (bind _returnvalue_4 (UserInterface|CreateWidget "/Game/Alchemist_main/Blueprints/ShopSystem/Shop_access.Shop_access_C"))
  (UserInterface|Viewport|AddtoViewport _returnvalue_4 0))

(fn ExitBed
  ;[1 1 1] play sound and unfade after waking up
  (Audio|PlaySound2D "/Game/Alchemist_main/Sound/SFX/birds_chirping.birds_chirping" 1.0 1.0 0.0 0 0)
  (CameraFades|StartCameraFade :self (Game|GetPlayerCameraManager 0) :FromAlpha 1.0 :Duration 2.0)
  (Utilities|Time|SetTimerbyFunctionName 0 "get up" 2.0))

(fn GetUp
  ;[1 1 1] Changes camera on wake up
  (Game|Player|SetViewTargetwithBlend (Game|GetPlayerController 0) (Game|GetPlayerCharacter 0) 0.0 "VTBlend_Linear" 0.0 false))

(fn GameOver
  (bind _returnvalue (Game|GetPlayerController 0))
  ;[1 1 1] Displays game over widget
  (bind _returnvalue_2 (UserInterface|CreateWidget "/Game/Alchemist_main/Blueprints/UISystem/MainAndPause/UI/menus/Final_screen.Final_screen_C" _returnvalue))
  (UserInterface|Viewport|AddtoViewport _returnvalue_2 0)
  (Variables|/Script/Engine.PlayerController|SetbShowMouseCursor _returnvalue true)
  (Input|SetInputModeUIOnly _returnvalue _returnvalue_2 "DoNotLock"))

(fn CheckGameOver
  (params (total%20unrest :type Integer))
  (bind _max_unrest (Variables|Default|GetMax%20unrest))
  (bind _returnvalue (> total%20unrest _max_unrest))
  ;[1 1 1] Checks whether the game is over
  (if _returnvalue
    (CallFunction|GameOver)
    (return _returnvalue)))

(fn CreateSleepMenus
  ;[1 1 1] fades camera and changes view and calls menu setup on sleep
  (Input|SetInputModeUIOnly (Game|GetPlayerController 0) 0 "DoNotLock")
  (Game|Player|SetViewTargetwithBlend (Game|GetPlayerController 0) self 0.0 "VTBlend_Linear" 0.0 false)
  (CameraFades|StartCameraFade :self (Game|GetPlayerCameraManager 0) :ToAlpha 1.0 :Duration 2.0 :bShouldFadeAudio true :bHoldWhenFinished true)
  (Utilities|Time|SetTimerbyFunctionName 0 "display town" 3.0))